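; BP_DogAIController is the AI controller for a dog, running the BT_DogAI behavior tree on possession.
; It stores the pawn's starting location in the blackboard on BeginPlay.
; Perception of a player-controlled pawn cancels the forget timer and sets the enemy and line-of-sight keys.
; Any other perception update starts that timer, which clears both keys after a LineOfSightTimer delay.
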(event `self.ReceiveBeginPlay`
  (`BlackboardComponent.SetValueAsVector` (`AIBlueprintHelperLibrary.GetBlackboard` null) (`self.OriginalPosition`) (`self.K2_GetActorLocation` (`self.K2_GetPawn`))))

(event `self.ReceivePossess`
  (params (PossessedPawn :type "Pawn Object Reference"))
  (`self.RunBehaviorTree` "/Game/Dog/BT_DogAI.BT_DogAI"))

(event `self.AIPerception.OnTargetPerceptionUpdated`
  (params (Actor :type "Actor Object Reference") (Stimulus :type "AIStimulus Structure"))
  (bind _returnvalue (`AIBlueprintHelperLibrary.GetBlackboard` null))
  (bind _aspawn (cast `Pawn` Actor)
    (:`then`
      (if (and (`Pawn.IsPlayerControlled` _aspawn) (`.bSuccessfullySensed` (break `AIStimulus` Stimulus)))
        (`KismetSystemLibrary.K2_ClearAndInvalidateTimerHandle` (`self.EnemyTimer`))
        (`BlackboardComponent.SetValueAsBool` _returnvalue (`self.HasLineOfSight`) true)
        (`BlackboardComponent.SetValueAsObject` _returnvalue (`self.EnemyActor`) Actor)
        (else
          (bind _returnvalue_2 (`KismetSystemLibrary.K2_SetTimerDelegate` (delegate `StartEnemy Timer`) (`self.LineOfSightTimer`) :!label _label))
          (set `self.EnemyTimer` _returnvalue_2))))
    (:`CastFailed`
      (goto _label))))

(event `StartEnemy Timer`
  (bind _returnvalue (`AIBlueprintHelperLibrary.GetBlackboard` null))
  (`BlackboardComponent.SetValueAsBool` _returnvalue (`self.HasLineOfSight`) false)
  (`BlackboardComponent.SetValueAsObject` _returnvalue (`self.EnemyActor`) null))

(fn `UserConstructionScript`)