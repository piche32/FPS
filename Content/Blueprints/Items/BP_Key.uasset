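; BP_Key is a key item actor that the player can hide and bring back with hard-coded keyboard events.
; V hides the actor and turns off its collision and mesh physics, with no proximity check.
; C teleports the actor to the first player pawn's location, then restores visibility, collision and physics.
; An unconnected alternative that moves only the mesh remains in the graph, and overlap and Tick do nothing.
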(event `Key|V`
  (params (Key :type "Key Structure"))
  (:`Pressed`
    (`self.SetActorHiddenInGame` true)
    (`self.SetActorEnableCollision` false)
    (`PrimitiveComponent.SetSimulatePhysics` (`self.Mesh`) false)))

(event `Key|C`
  (params (Key :type "Key Structure"))
  (:`Pressed`
    (`self.K2_SetActorLocation` (`self.K2_GetActorLocation` (`GameplayStatics.GetPlayerPawn` 0)) false true)
    (`self.SetActorHiddenInGame` false)
    (`self.SetActorEnableCollision` true)
    (`PrimitiveComponent.SetSimulatePhysics` (`self.Mesh`) true)))

(fn `UserConstructionScript`)