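; BP_FakeWall is a fake wall built on a Geometry Collection, with child-actor anchor fields attached to it.
; The Construction Script loops over three child actor components, casts each spawned actor to FS_AnchorField_Generic and adds it to the collection's InitializationFields.
; BeginPlay is empty, and an older four-field version of the same registration sits disconnected in the EventGraph.
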(event `self.ReceiveBeginPlay`)

(fn `UserConstructionScript`
  (for _array_element (`|MakeArray` (`self.AnchorField1`) (`self.AnchorField3`) (`self.AnchorField2`))
    (bind _asfs_anchor_field_generic (cast `/Engine/EditorResources/FieldNodes/FS_AnchorField_Generic` (`ChildActorComponent.ChildActor` _array_element)))
    (`KismetArrayLibrary.Array_Add` (`GeometryCollectionComponent.InitializationFields` (`self.BP_FakeWall_GeometryCollection`)) _asfs_anchor_field_generic)))