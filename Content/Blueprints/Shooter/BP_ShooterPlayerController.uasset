(event `Key|I`
  (params (Key :type "Key Structure"))
  ;[1 1 1] Toggle Inventory Menu
  (:`Pressed`
    (if (not (`self.InventoryDelay_BP`))
      (bind _aswbp_hud (cast `/Game/UI/WBP_HUD` (`self.HUD`)))
      (if (`/Game/UI/WBP_HUD.ActivateInventory` _aswbp_hud)
        (`/Engine/EditorBlueprintResources/StandardMacros.FlipFlop`
          (:`A`
            (set `/Game/UI/WBP_HUD.InventoryVisible` "Visible" _aswbp_hud)
            (`self.EnableMouseCursor`)
            (bind _aswbp_hud_2 (cast `/Game/UI/WBP_HUD` (`self.HUD`)))
            (`UserWidget.PlayAnimation` _aswbp_hud_2 (`/Game/UI/WBP_HUD.MenuAnim` _aswbp_hud_2) 0.0 1 "Forward" 1.0 false)
            (set `self.InventoryDelay_BP` true)
            (set `self.MenuOpen_BP` true))
          (:`B`
            (set `self.InventoryDelay_BP` true)
            (bind _aswbp_hud_3 (cast `/Game/UI/WBP_HUD` (`self.HUD`)))
            (`UserWidget.PlayAnimation` _aswbp_hud_3 (`/Game/UI/WBP_HUD.MenuAnim` _aswbp_hud_3) 0.0 1 "Reverse" 1.0 false)
            (`KismetSystemLibrary.Delay` 0.7)
            (set `/Game/UI/WBP_HUD.InventoryVisible` "Hidden" _aswbp_hud)
            (`self.DisableMouseCursor`)
            (set `self.MenuOpen_BP` false)))
        (`KismetSystemLibrary.Delay` 0.5)
        (set `self.InventoryDelay_BP` false)))))

(event `Key|F`
  (params (Key :type "Key Structure"))
  (:`Pressed`
    (`/Engine/EditorBlueprintResources/StandardMacros.FlipFlop`
      (:`A`
        (`self.EnableMouseCursor`))
      (:`B`
        (`self.DisableMouseCursor`)))))

(event `Key|E`
  (params (Key :type "Key Structure"))
  ;[1 1 1] Pickup Items
  (:`Pressed`
    (bind _aswbp_hud (cast `/Game/UI/WBP_HUD` (`self.HUD`)))
    (if (< (`KismetArrayLibrary.Array_Length` (`/Game/UI/WBP_HUD.Inventory_BP` _aswbp_hud)) 5)
      (`self.PickupItem`))))

(event `/Game/UI/BP_ItemActionInterface.DropAction`
  (params (`Item To Drop` :type "Actor Object Reference"))
  ;[1 1 1] Drop Items
  (bind _asbp_shooter (cast `/Game/Blueprints/Shooter/BP_Shooter` (`self.K2_GetPawn`)))
  (`self.SetActorHiddenInGame` `Item To Drop` false)
  (`self.SetActorEnableCollision` `Item To Drop` true)
  (`self.K2_SetActorTransform` `Item To Drop` (`SceneComponent.K2_GetComponentToWorld` (`/Game/Blueprints/Shooter/BP_Shooter.DropLocation` _asbp_shooter)) false false))

(event `/Game/UI/BP_ItemActionInterface.UseAction`)

(fn `DisableMouseCursor`
  (bind _aswbp_hud (cast `/Game/UI/WBP_HUD` (`self.HUD`)))
  (`WidgetBlueprintLibrary.SetInputMode_GameOnly` self)
  (set `/Game/UI/WBP_HUD.ShowCrosshairs` true _aswbp_hud)
  (set `self.bShowMouseCursor` false))

(fn `EnableMouseCursor`
  (bind _aswbp_hud (cast `/Game/UI/WBP_HUD` (`self.HUD`)))
  (`WidgetBlueprintLibrary.SetInputMode_GameAndUIEx` self _aswbp_hud)
  (set `/Game/UI/WBP_HUD.ShowCrosshairs` false _aswbp_hud)
  (set `self.bShowMouseCursor` true))

(fn `UserConstructionScript`)