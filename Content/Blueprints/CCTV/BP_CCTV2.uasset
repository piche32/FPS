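; CCTV security turret whose top mesh sweeps back and forth within a yaw limit and damages targets with a laser beam.
; Rotate, attack and beam-update functions are exposed here, with no callers in this Blueprint.
; When damage leaves its HealthComponent dead, it swaps laser for smoke, detaches its controller and tips the top over via a looping timer.
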(event `self.ReceiveBeginPlay`
  (add `self.OnTakeAnyDamage` (delegate `OnTakeAnyDamage_Event`))
  (`ActorComponent.Deactivate` (`self.SmokeSystem_BP`)))

(event `OnTakeAnyDamage_Event` :!signature `self.OnTakeAnyDamage`
  (params (DamagedActor :type "Actor Object Reference") (Damage :type "Float (single-precision)") (DamageType :type "DamageType Object Reference") (InstigatedBy :type "Controller Object Reference") (DamageCauser :type "Actor Object Reference"))
  (if (`HealthComponent.IsDead` (`self.HealthComponent`))
    (`self.OnDead_BP`)))

(fn `Attack_BP`
  (params (DamagedActor :type "Actor Object Reference"))
  (`|ExecutionSequence`
    (:`then_0`
      (`GameplayStatics.ApplyDamage` DamagedActor (`self.Damage_BP`) (`self.GetController`) self "/Script/Engine.DamageType"))
    (:`then_1`
      (`self.UpdateLaser_BP` (`self.K2_GetActorLocation` DamagedActor)))))

(fn `DeadMotion_BP`
  (bind _topmesh (`self.TopMesh`))
  (bind (_relativerotation_roll _relativerotation_pitch _relativerotation_yaw) (`KismetMathLibrary.BreakRotator` (`SceneComponent.RelativeRotation` _topmesh)))
  (bind _relativerotation_roll_2 (`KismetMathLibrary.BreakRotator` (`SceneComponent.RelativeRotation` _topmesh)))
  (`SceneComponent.K2_SetRelativeRotation` _topmesh (`KismetMathLibrary.RInterpTo` (`SceneComponent.RelativeRotation` _topmesh) (`KismetMathLibrary.MakeRotator` -90.0 _relativerotation_pitch _relativerotation_yaw) (`GameplayStatics.GetWorldDeltaSeconds`) 1.0) false false)
  (if (`KismetMathLibrary.InRange_FloatFloat` _relativerotation_roll_2 -87.0 -93.0)
    (`KismetSystemLibrary.K2_ClearAndInvalidateTimerHandle` (`self.DeadTimer_BP`))))

(fn `OnDead_BP`
  (`|ExecutionSequence`
    (:`then_0`
      (bind _returnvalue (`KismetSystemLibrary.K2_SetTimer` null "DeadMotion_BP" (`GameplayStatics.GetWorldDeltaSeconds`) true))
      (set `self.DeadTimer_BP` _returnvalue))
    (:`then_1`
      (`ActorComponent.Deactivate` (`self.LaserBeamSystem_BP`)))
    (:`then_2`
      (`ActorComponent.Activate` (`self.SmokeSystem_BP`) false))
    (:`then_3`
      (`self.DetachFromControllerPendingDestroy`))))

(fn `Rotate_BP`
  (params (DeltaTime :type "Float (double-precision) (by ref)"))
  (bind _topmesh (`self.TopMesh`))
  (bind _maxangle (`self.MaxAngle`))
  (bind (_relativerotation_roll _relativerotation_pitch _relativerotation_yaw) (`KismetMathLibrary.BreakRotator` (`SceneComponent.RelativeRotation` _topmesh)))
  (bind _returnvalue (+ _relativerotation_yaw (* (`self.RotVelocity`) DeltaTime)))
  (`SceneComponent.K2_SetRelativeRotation` _topmesh (`KismetMathLibrary.MakeRotator` _relativerotation_roll _relativerotation_pitch _returnvalue) false false)
  (if (not (`KismetMathLibrary.InRange_FloatFloat` _returnvalue (- 0.0 _maxangle) _maxangle))
    (set `self.RotVelocity` (* (`self.RotVelocity`) -1.0))))

(fn `UpdateLaser_BP`
  (params (Target :type "Vector Structure"))
  (`FXSystemComponent.SetVectorParameter` (`self.LaserBeamSystem_BP`) "Beam End" Target))

(fn `UserConstructionScript`)